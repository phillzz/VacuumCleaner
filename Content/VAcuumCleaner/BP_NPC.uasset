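; NPC character Blueprint that reacts to zero-gravity and vacuum bomb effects through custom events.
; Zero gravity launches the NPC gently upward and restores gravity after a timed delay.
; The vacuum bomb disables gravity, then after a delay a timeline lerps the NPC toward the first VacuumBomb found, shrinking it and stopping mesh animation.
; Deactivation restores gravity and drives scale through a second timeline.
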(event EventActivateVacuumBomb
  (bind _mesh (Variables|Character|GetMesh))
  (Variables|/Script/Engine.CharacterMovementComponent|SetGravityScale (Variables|Character|GetCharacterMovement) 0.0)
  (Utilities|FlowControl|Delay 2.0)
  (bind _outactors (Actor|GetAllActorsOfClass "/Game/VAcuumCleaner/VacuumBomb.VacuumBomb_C"))
  (bind _newtrack_0 (Timeline|Timeline_0 Play)
    (:Update
      (Transformation|SetActorLocation (Math|Vector|Lerp(Vector) (Transformation|GetActorLocation) (Transformation|GetActorLocation (Utilities|Array|Get(acopy) _outactors)) _newtrack_0) false false)
      (Transformation|SetActorScale3D (Math|Vector|Lerp(Vector) "1.000000,1.000000,1.000000" "0.200000,0.200000,0.200000" _newtrack_0))
      (if (Audio|Components|Audio|IsPlaying _mesh)
        (Audio|Components|Audio|Stop _mesh)))))

(event EventDeactivateVacuumBomb
  (Variables|/Script/Engine.CharacterMovementComponent|SetGravityScale (Variables|Character|GetCharacterMovement) 1.0)
  (bind _newtrack_0 (Timeline|Timeline_1 Play)
    (:Update
      (Transformation|SetActorScale3D (Math|Vector|Lerp(Vector) "1.000000,1.000000,1.000000" "0.200000,0.200000,0.200000" _newtrack_0)))))

(event EventActivateZeroGravity
  (bind _charactermovement (Variables|Character|GetCharacterMovement))
  (Variables|/Script/Engine.CharacterMovementComponent|SetGravityScale _charactermovement 0.0)
  (Character|LaunchCharacter "0, 0,70.000000" false false)
  (Utilities|FlowControl|Delay 7.0)
  (Variables|/Script/Engine.CharacterMovementComponent|SetGravityScale _charactermovement 1.0))

(fn ConstructionScript
  (|CallParentFunction))